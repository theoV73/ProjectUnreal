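; Laser tower that targets the player inside a 30-degree cone in front of its shoot point.
; Each tick it traces WorldStatic toward the player; a blocking hit rotates the pivot, ends the laser on the player and fires the PlayerHealth dispatcher.
; Otherwise a forward trace sets the laser's end through the EndLaser effect parameter.
; The tower's own PlayerHealth handler is empty, and both traces draw persistent debug lines.
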(event `self.ReceiveBeginPlay`
  (set `self.Damages` 1.0)
  (add `self.PlayerHealth` (delegate `PlayerHealth_Event`)))

(event `PlayerHealth_Event`)

(event `self.ReceiveTick`
  (params (DeltaSeconds :type "Float (single-precision)"))
  (bind _shootpoint (`self.ShootPoint`))
  (bind _shootpoint_2 (`self.ShootPoint`))
  (bind _returnvalue (`SceneComponent.K2_GetComponentLocation` _shootpoint))
  (bind _returnvalue_2 (`SceneComponent.K2_GetComponentLocation` (`self.ShootPoint`)))
  (bind _returnvalue_3 (`SceneComponent.K2_GetComponentLocation` (`Actor.RootComponent` (`GameplayStatics.GetPlayerCharacter` 0))))
  (if (<= (`KismetMathLibrary.DegAcos` (`KismetMathLibrary.Dot_VectorVector` (`SceneComponent.GetForwardVector` _shootpoint_2) (`KismetMathLibrary.Normal` (- _returnvalue_3 (`SceneComponent.K2_GetComponentLocation` _shootpoint_2))))) 30.0)
    (bind _outhit (`KismetSystemLibrary.LineTraceSingleForObjects` :`Start` _returnvalue_2 :`End` _returnvalue_3 :`ObjectTypes` (`|MakeArray` "ObjectTypeQuery1" :!type "EObjectTypeQuery Enum") :`DrawDebugType` "Persistent"))
    (if (`GameplayStatics.BreakHitResult` _outhit)
      (`SceneComponent.K2_SetWorldRotation` (`self.Pivot`) (`KismetMathLibrary.FindLookAtRotation` _returnvalue_2 _returnvalue_3) false false)
      (`FXSystemComponent.SetVectorParameter` (`self.Projectile`) "EndLaser" _returnvalue_3)
      (`self.PlayerHealth`)
      (else
        (bind _outhit_2 (`KismetSystemLibrary.LineTraceSingleForObjects` :`Start` _returnvalue :`End` (+ _returnvalue (* (`SceneComponent.GetForwardVector` _shootpoint) 1000.0)) :`ObjectTypes` (`|MakeArray` "ObjectTypeQuery1" :!type "EObjectTypeQuery Enum") :`DrawDebugType` "Persistent" :!label _label))
        (`FXSystemComponent.SetVectorParameter` (`self.Projectile`) "EndLaser" (`.Location` (`GameplayStatics.BreakHitResult` _outhit_2)))))
    (else
      (goto _label))))

(fn `UserConstructionScript`)