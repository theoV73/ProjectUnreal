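; BP_Tower is a laser turret that tracks and damages the player within a 30-degree cone of its shoot point.
; Each Tick it traces to the player, turns its pivot and moves the laser effect's endpoint, or otherwise traces forward against world geometry.
; A first-person character hit loses Damages per frame through SetHealth, which updates the health bar or sets IsDead.
; Debug traces and prints remain, while timer and event-binding nodes are unwired.
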(event `self.ReceiveBeginPlay`)

(event `PlayerHealth_Event`)

(event `self.ReceiveTick`
  (params (DeltaSeconds :type "Float (single-precision)"))
  (bind _shootpoint (`self.ShootPoint`))
  (bind _shootpoint_2 (`self.ShootPoint`))
  (bind _returnvalue (`SceneComponent.K2_GetComponentLocation` _shootpoint))
  (bind _returnvalue_2 (`SceneComponent.K2_GetComponentLocation` (`self.ShootPoint`)))
  (bind _returnvalue_3 (`SceneComponent.K2_GetComponentLocation` (`Actor.RootComponent` (`GameplayStatics.GetPlayerCharacter` 0))))
  (if (<= (`KismetMathLibrary.DegAcos` (`KismetMathLibrary.Dot_VectorVector` (`SceneComponent.GetForwardVector` _shootpoint_2) (`KismetMathLibrary.Normal` (- _returnvalue_3 (`SceneComponent.K2_GetComponentLocation` _shootpoint_2))))) 30.0)
    (bind _outhit (`KismetSystemLibrary.LineTraceSingleForObjects` :`Start` _returnvalue_2 :`End` _returnvalue_3 :`ObjectTypes` (`|MakeArray` "ObjectTypeQuery1" "ObjectTypeQuery3" "ObjectTypeQuery4" :!type "EObjectTypeQuery Enum") :`DrawDebugType` "Persistent"))
    (`SceneComponent.K2_SetWorldRotation` (`self.Pivot`) (`KismetMathLibrary.FindLookAtRotation` _returnvalue_2 _returnvalue_3) false false)
    (`FXSystemComponent.SetVectorParameter` (`self.Projectile`) "EndLaser" _returnvalue_3)
    (bind _asbp_first_person_character (cast `/Game/FirstPerson/Blueprints/BP_FirstPersonCharacter` (`.HitActor` (`GameplayStatics.BreakHitResult` _outhit))))
    (bind _health (`self.SetHealth` _asbp_first_person_character))
    (bind _output_get (set `/Game/FirstPerson/Blueprints/BP_FirstPersonCharacter.Health` _health _asbp_first_person_character))
    (`KismetSystemLibrary.PrintString` (`KismetStringLibrary.Conv_DoubleToString` _output_get))
    (else
      (bind _outhit_2 (`KismetSystemLibrary.LineTraceSingleForObjects` :`Start` _returnvalue :`End` (+ _returnvalue (* (`SceneComponent.GetForwardVector` _shootpoint) 1000.0)) :`ObjectTypes` (`|MakeArray` "ObjectTypeQuery1" :!type "EObjectTypeQuery Enum") :`DrawDebugType` "Persistent"))
      (`FXSystemComponent.SetVectorParameter` (`self.Projectile`) "EndLaser" (`.Location` (`GameplayStatics.BreakHitResult` _outhit_2))))))

(fn `SetHealth`
  (params (Player :type "/Game/FirstPerson/Blueprints/BP_FirstPersonCharacter Object Reference"))
  (returns (Health :type "Float (double-precision)"))
  (bind _returnvalue (- (`/Game/FirstPerson/Blueprints/BP_FirstPersonCharacter.Health` Player) (`self.Damages`)))
  (if (<= _returnvalue 0.0)
    (set `/Game/FirstPerson/Blueprints/BP_FirstPersonCharacter.IsDead` true Player)
    (`KismetSystemLibrary.PrintString` "Dead : ")
    (else
      (bind _output_get (set `/Game/Blueprint/BPW_Player_Interface.HealthBar` _returnvalue (`/Game/FirstPerson/Blueprints/BP_FirstPersonCharacter.InterfaceHealth` Player)))
      (`KismetSystemLibrary.PrintString` "Alife : ")))
  (`KismetSystemLibrary.PrintString` (`KismetStringLibrary.Conv_DoubleToString` _output_get))
  (return _returnvalue))

(fn `UserConstructionScript`)