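; Dungeon room actor that randomly populates itself with a chest (Coffre), a tower (BP_Tower) or nothing.
; On BeginPlay it rolls one of four outcomes, two of which spawn an actor slightly above the room's origin, keeping its rotation and scale.
; An unconnected branch for randomly spawning BP_End is present but never runs.
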(event `self.ReceiveBeginPlay`
  (bind _spawn_transform (`self.Spawn Transform`))
  (bind (_spawn_transform_location _spawn_transform_rotation _spawn_transform_scale) (`KismetMathLibrary.BreakTransform` (`self.Spawn Transform`)))
  (bind _output_get (set `self.Spawn Transform` (`self.GetTransform`)))
  (bind _output_get_2 (set `self.Position` (`KismetMathLibrary.MakeVector` (.x (.location _output_get)) (.y (.location _output_get)) (+ (.z (.location _output_get)) 100.0))))
  (set `self.Spawn Transform` (`KismetMathLibrary.MakeTransform` _output_get_2 _spawn_transform_rotation _spawn_transform_scale))
  (bind _output_get_3 (set `self.valueRandom` (`KismetMathLibrary.RandomInteger` 4)))
  (switch `int` _output_get_3
    (:`0`
      (`|SpawnActorFromClass` "/Game/Blueprint/Dungeon/Coffre.Coffre_C" _spawn_transform "AdjustIfPossibleButAlwaysSpawn" "MultiplyWithRoot" null null))
    (:`1`
      (`|SpawnActorFromClass` "/Game/Blueprint/BP_Tower.BP_Tower_C" _spawn_transform "Undefined" "MultiplyWithRoot" null null))))

(fn `UserConstructionScript`)