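; Dungeon generator that builds a random chain of corridors and rooms on BeginPlay.
; A fixed-length loop random-walks SpawnPosition in four horizontal directions, spawning a Corridor one step away and a Room another step beyond.
; Directional helpers orient corridors, while SpawnRoomX and SpawnRoomZ advance along X and Y respectively.
; PreviousChoice is stored but never read, so paths can double back; the CorridorAngle branch is unwired.
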(event `self.ReceiveBeginPlay`
  (bind _valueloop (`self.ValueLoop`))
  (bind (_spawnposition_x _spawnposition_y _spawnposition_z) (`KismetMathLibrary.BreakVector` (`self.SpawnPosition`)))
  (bind (_spawnposition_x_2 _spawnposition_y_2 _spawnposition_z_2) (`KismetMathLibrary.BreakVector` (`self.SpawnPosition`)))
  (bind (_spawnposition_x_3 _spawnposition_y_3 _spawnposition_z_3) (`KismetMathLibrary.BreakVector` (`self.SpawnPosition`)))
  (bind (_spawnposition_x_4 _spawnposition_y_4 _spawnposition_z_4) (`KismetMathLibrary.BreakVector` (`self.SpawnPosition`)))
  (while (< _valueloop 10)
    (set `self.ValueLoop` (+ _valueloop 1))
    (bind _output_get (set `self.Choice` (`KismetMathLibrary.RandomInteger` 4)))
    (switch `int` _output_get
      (:`0`
        (bind _output_get_2 (set `self.SpawnPosition` (`KismetMathLibrary.MakeVector` (+ _spawnposition_x_3 1000.0) _spawnposition_y_3 _spawnposition_z_3)))
        (`self.CorridorFront` _output_get_2)
        (`self.SpawnRoomX` 1000.0))
      (:`1`
        (bind _output_get_3 (set `self.SpawnPosition` (`KismetMathLibrary.MakeVector` (+ _spawnposition_x -1000.0) _spawnposition_y _spawnposition_z)))
        (`self.CorridorBack` _output_get_3)
        (`self.SpawnRoomX` -1000.0))
      (:`2`
        (bind _output_get_4 (set `self.SpawnPosition` (`KismetMathLibrary.MakeVector` _spawnposition_x_2 (+ 1000.0 _spawnposition_y_2) _spawnposition_z_2)))
        (`self.CorridorRight` _output_get_4)
        (`self.SpawnRoomZ` 1000.0))
      (:`3`
        (bind _output_get_5 (set `self.SpawnPosition` (`KismetMathLibrary.MakeVector` _spawnposition_x_4 (+ _spawnposition_y_4 -1000.0) _spawnposition_z_4)))
        (`self.CorridorLeft` _output_get_5)
        (`self.SpawnRoomZ` -1000.0)))
    (set `self.PreviousChoice` (`self.Choice`))))

(fn `CorridorBack`
  (params (trans_Location :type "Vector Structure"))
  (bind _output_get (set `self.SpawnRotation` (0.0 0.0 0.0)))
  (bind _output_get_2 (set `self.trans` (`KismetMathLibrary.MakeTransform` trans_Location (`KismetMathLibrary.Conv_VectorToRotator` _output_get))))
  (`|SpawnActorFromClass` "/Game/Blueprint/Dungeon/Corridor.Corridor_C" _output_get_2 "AdjustIfPossibleButAlwaysSpawn" "MultiplyWithRoot" null null))

(fn `CorridorFront`
  (params (trans_Location :type "Vector Structure"))
  (bind _output_get (set `self.SpawnRotation` (0.0 0.0 0.0)))
  (bind _output_get_2 (set `self.trans` (`KismetMathLibrary.MakeTransform` trans_Location (`KismetMathLibrary.Conv_VectorToRotator` _output_get))))
  (`|SpawnActorFromClass` "/Game/Blueprint/Dungeon/Corridor.Corridor_C" _output_get_2 "AdjustIfPossibleButAlwaysSpawn" "MultiplyWithRoot" null null))

(fn `CorridorLeft`
  (params (trans_Location :type "Vector Structure"))
  (bind _output_get (set `self.SpawnRotation` (0.0 -90.0 0.0)))
  (bind _output_get_2 (set `self.trans` (`KismetMathLibrary.MakeTransform` trans_Location (`KismetMathLibrary.Conv_VectorToRotator` _output_get))))
  (`|SpawnActorFromClass` "/Game/Blueprint/Dungeon/Corridor.Corridor_C" _output_get_2 "AdjustIfPossibleButAlwaysSpawn" "MultiplyWithRoot" null null))

(fn `CorridorRight`
  (params (trans_Location :type "Vector Structure"))
  (bind _output_get (set `self.SpawnRotation` (0.0 90.0 0.0)))
  (bind _output_get_2 (set `self.trans` (`KismetMathLibrary.MakeTransform` trans_Location (`KismetMathLibrary.Conv_VectorToRotator` _output_get))))
  (`|SpawnActorFromClass` "/Game/Blueprint/Dungeon/Corridor.Corridor_C" _output_get_2 "AdjustIfPossibleButAlwaysSpawn" "MultiplyWithRoot" null null))

(fn `Debug`
  (params (valueLoop :type Integer))
  (`KismetSystemLibrary.PrintString` (`KismetStringLibrary.Conv_IntToString` valueLoop)))

(fn `SpawnRoomX`
  (params (Distance :type "Float (double-precision)"))
  (bind (_spawnposition_x _spawnposition_y _spawnposition_z) (`KismetMathLibrary.BreakVector` (`self.SpawnPosition`)))
  (bind _output_get (set `self.SpawnPosition` (`KismetMathLibrary.MakeVector` (+ _spawnposition_x Distance) _spawnposition_y _spawnposition_z)))
  (`|SpawnActorFromClass` "/Game/Blueprint/Dungeon/Room.Room_C" (`KismetMathLibrary.Conv_VectorToTransform` _output_get) "AdjustIfPossibleButAlwaysSpawn" "MultiplyWithRoot" null null)
  (return))

(fn `SpawnRoomZ`
  (params (Distance :type "Float (double-precision)"))
  (bind (_spawnposition_x _spawnposition_y _spawnposition_z) (`KismetMathLibrary.BreakVector` (`self.SpawnPosition`)))
  (bind _output_get (set `self.SpawnPosition` (`KismetMathLibrary.MakeVector` _spawnposition_x (+ Distance _spawnposition_y) _spawnposition_z)))
  (`|SpawnActorFromClass` "/Game/Blueprint/Dungeon/Room.Room_C" (`KismetMathLibrary.Conv_VectorToTransform` _output_get) "AdjustIfPossibleButAlwaysSpawn" "MultiplyWithRoot" null null)
  (return))

(fn `UserConstructionScript`)